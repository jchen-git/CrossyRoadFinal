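; Rail Blueprint that spawns trains and crossing lights along a railway.
; On BeginPlay it caches the transforms of two spawn components and places a crossing lights actor at each of two crossing components.
; Each Tick spawns a train at a randomly chosen spawn point with a sound at that location, then randomizes its own tick interval so trains arrive at irregular gaps of several seconds.
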(event `self.ReceiveBeginPlay`
  (set `self.SpawnLoc` (`|MakeArray` (`SceneComponent.K2_GetComponentToWorld` (`self.spawn1`)) (`SceneComponent.K2_GetComponentToWorld` (`self.spawn2`))))
  (`|SpawnActorFromClass` "/Game/Blueprints/crossing_lights_Blueprint.crossing_lights_Blueprint_C" (`SceneComponent.K2_GetComponentToWorld` (`self.crossing1`)) "Undefined" "OverrideRootScale" null null)
  (`|SpawnActorFromClass` "/Game/Blueprints/crossing_lights_Blueprint.crossing_lights_Blueprint_C" (`SceneComponent.K2_GetComponentToWorld` (`self.crossing2`)) "Undefined" "OverrideRootScale" null null))

(event `self.ReceiveTick`
  (params (DeltaSeconds :type "Float (single-precision)"))
  (bind _output_get (set `self.StartLoc` (`KismetArrayLibrary.Array_Random` (`self.SpawnLoc`))))
  (`|SpawnActorFromClass` "/Game/Blueprints/train.train_C" _output_get "Undefined" "OverrideRootScale" null null)
  (`GameplayStatics.PlaySoundAtLocation` "/Game/Sounds/train.train" (.location _output_get) (struct) 1.0 1.0 0.0 null null null null)
  (`self.SetActorTickInterval` (`KismetMathLibrary.RandomFloatInRange` 8.0 13.0)))

(fn `UserConstructionScript`)