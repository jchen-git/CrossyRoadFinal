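; Crossing light Blueprint meant to switch between red and blue states.
; ChangeRed and ChangeBlue each recolor the SpotLight and toggle visibility of the Red and Blue components.
; Tick sets looping timers by function name for both changes every frame, restarting their countdowns, with identical intervals and no offset between colors.
; An unconnected branch hides both components.
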(event `self.ReceiveTick`
  (params (DeltaSeconds :type "Float (single-precision)"))
  (`KismetSystemLibrary.K2_SetTimer` null "Change Blue" 1.5 true)
  (`KismetSystemLibrary.K2_SetTimer` null "Change Red" 1.5 true))

(event `Change Red`
  (`LightComponent.SetLightColor` (`self.SpotLight`) (struct :`R` 1.0 :`G` 0.016606 :`A` 1.0) true)
  (`SceneComponent.SetVisibility` (`self.red`) true false)
  (`SceneComponent.SetVisibility` (`self.blue`) false false))

(event `Change Blue`
  (`LightComponent.SetLightColor` (`self.SpotLight`) (struct :`G` 0.027924 :`B` 1.0 :`A` 1.0) true)
  (`SceneComponent.SetVisibility` (`self.red`) false false)
  (`SceneComponent.SetVisibility` (`self.blue`) true false))

(fn `UserConstructionScript`)