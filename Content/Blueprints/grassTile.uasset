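; Grass tile actor that randomly populates itself with props and pickups when play begins.
; On BeginPlay it gathers the world transforms of five spawn-point components and rolls for each one.
; Most points stay empty; a chain of successive random checks picks a Rock, a SmallTree, a Coin or nothing, making rocks the most common spawn and coins rarer.
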(event `self.ReceiveBeginPlay`
  (bind _output_get (set `self.spawnLoc` (`|MakeArray` (`SceneComponent.K2_GetComponentToWorld` (`self.spawn1`)) (`SceneComponent.K2_GetComponentToWorld` (`self.spawn2`)) (`SceneComponent.K2_GetComponentToWorld` (`self.spawn3`)) (`SceneComponent.K2_GetComponentToWorld` (`self.spawn4`)) (`SceneComponent.K2_GetComponentToWorld` (`self.spawn5`)))))
  (for _array_element _output_get
    (if (> (`KismetMathLibrary.RandomIntegerInRange` 0 100) 60)
      (if (> (`KismetMathLibrary.RandomIntegerInRange` 0 100) 50)
        (`|SpawnActorFromClass` "/Game/Blueprints/rock.rock_C" _array_element "Undefined" "OverrideRootScale" null null)
        (elif (> (`KismetMathLibrary.RandomIntegerInRange` 0 100) 50)
          (`|SpawnActorFromClass` "/Game/Blueprints/SmallTree.SmallTree_C" _array_element "Undefined" "OverrideRootScale" null null)
          (elif (> (`KismetMathLibrary.RandomIntegerInRange` 0 100) 50)
            (`|SpawnActorFromClass` "/Game/Blueprints/coin.coin_C" _array_element "Undefined" "OverrideRootScale" null null)))))))

(fn `UserConstructionScript`)