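; Player character for a Frogger-style game, a chicken that hops between obstacles and dies on contact with vehicle- or water-tagged actors.
; Key-to-value maps set each hop's offset and facing, and a timeline lerps the swept move, ignoring new hops while playing.
; W presses add score while alive, independently of hop completion.
; Death hides the mesh, disables collision and saves any new high score; R then reloads Map1.
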(event `self.ReceiveBeginPlay`
  (bind _returnvalue (`|CreateWidget` "/Game/Blueprints/HUDBlueprint.HUDBlueprint_C"))
  (bind _output_get (set `self.HUD Reference` _returnvalue))
  (`UserWidget.AddToViewport` _output_get 0)
  (set `self.Splash` "/Game/Effects/Splash.Splash")
  (bind _returnvalue_2 (`GameplayStatics.DoesSaveGameExist` "slot 0"))
  (if _returnvalue_2
    (bind _returnvalue_3 (`GameplayStatics.LoadGameFromSlot` "slot 0"))
    (bind _output_get_2 (set `self.Save Sub Class` _returnvalue_3))
    (bind _assave_game_hs (cast `/Game/Blueprints/saveGameHS` _output_get_2))
    (set `self.High Score` (`/Game/Blueprints/saveGameHS.High Score` _assave_game_hs))
    (else
      (bind _returnvalue_4 (`GameplayStatics.CreateSaveGameObject` "/Game/Blueprints/saveGameHS.saveGameHS_C"))
      (bind _output_get_3 (set `self.Save Sub Class` _returnvalue_4))
      (cast `/Game/Blueprints/saveGameHS` _output_get_3)
      (set `self.High Score` 0))))

(event `self.ReceiveActorBeginOverlap`
  (params (OtherActor :type "Actor Object Reference"))
  ;[1 1 1] Obstacle Collision
  (if (`self.ActorHasTag` OtherActor "vehicle")
    (`GameplayStatics.PlaySound2D` "/Game/Sounds/chicken_die.chicken_die" 1.0 1.0 0.0 null null)
    (`/Engine/EditorBlueprintResources/StandardMacros.DoOnce` false :!label _label
      (:`Completed`
        (`SceneComponent.SetVisibility` (`self.Mesh`) false false)
        (`PrimitiveComponent.SetCollisionEnabled` (`self.Mesh`) "NoCollision")
        (`PrimitiveComponent.SetCollisionEnabled` (`self.CapsuleComponent`) "NoCollision")
        (set `self.alive` false)
        (if (> (`self.Score`) (`self.High Score`))
          (set `self.High Score` (`self.Score`))
          (bind _returnvalue (`GameplayStatics.DoesSaveGameExist` "slot 0"))
          (if _returnvalue
            (bind _returnvalue_2 (`GameplayStatics.LoadGameFromSlot` "slot 0"))
            (bind _output_get (set `self.Save Sub Class` _returnvalue_2))
            (bind _assave_game_hs (cast `/Game/Blueprints/saveGameHS` _output_get))
            (set `/Game/Blueprints/saveGameHS.High Score` (`self.High Score`) _assave_game_hs)
            (`GameplayStatics.SaveGameToSlot` (`self.Save Sub Class`) "slot 0")
            (else
              (bind _returnvalue_3 (`GameplayStatics.CreateSaveGameObject` "/Game/Blueprints/saveGameHS.saveGameHS_C"))
              (bind _output_get_2 (set `self.Save Sub Class` _returnvalue_3))
              (bind _assave_game_hs_2 (cast `/Game/Blueprints/saveGameHS` _output_get_2))
              (set `/Game/Blueprints/saveGameHS.High Score` (`self.High Score`) _assave_game_hs_2)
              (`GameplayStatics.SaveGameToSlot` (`self.Save Sub Class`) "slot 0"))))))
    (elif (`self.ActorHasTag` OtherActor "water")
      (`GameplayStatics.PlaySound2D` "/Game/Sounds/splash.splash" 1.0 1.0 0.0 null null)
      (`NiagaraFunctionLibrary.SpawnSystemAtLocation` (`self.Splash`) (`self.endLoc`))
      (goto _label))))

(event `Key|AnyKey`
  (params (Key :type "Key Structure"))
  (bind (_value _returnvalue) (`BlueprintMapLibrary.Map_Find` (`self.directionKeys`) Key))
  ;[1 1 1] Movement
  (:`Pressed`
    (if (and (`self.alive`) _returnvalue)
      (if (not (`TimelineComponent.IsPlaying` (`self.Timeline`)))
        (bind _output_get (set `self.startLoc` (`self.K2_GetActorLocation`)))
        (bind _output_get_2 (set `self.endLoc` (+ _output_get (`KismetMathLibrary.MakeVector` (`BlueprintMapLibrary.Map_Find` (`self.moveForward`) Key) (`BlueprintMapLibrary.Map_Find` (`self.moveRight`) Key) 40.0))))
        (`GameplayStatics.PlaySoundAtLocation` "/Game/Sounds/chicken.chicken" _output_get_2 (struct) 1.0 1.0 0.0 null null null null)
        (bind (_direction _move_alpha) (`Timeline|Timeline` :!via `PlayFromStart`)
          (:`Update`
            (`SceneComponent.K2_SetWorldRotation` (`self.Mesh`) (`KismetMathLibrary.MakeRotator` 0.0 0.0 _value) false false)
            (`self.K2_SetActorLocation` (`KismetMathLibrary.VLerp` (`self.startLoc`) (`self.endLoc`) _move_alpha) true)))))))

(event `Key|W`
  (params (Key :type "Key Structure"))
  (:`Pressed`
    (if (`self.alive`)
      (`/Engine/EditorBlueprintResources/StandardMacros.IncrementInt` (`self.Score`)))))

(event `Key|R`
  (params (Key :type "Key Structure"))
  (:`Pressed`
    (if (not (`self.alive`))
      (`GameplayStatics.OpenLevel` "Map1"))))

(fn `UserConstructionScript`)