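; Road actor that spawns random traffic vehicles at irregular intervals.
; On BeginPlay it builds lists of vehicle classes (police, regular car, truck) and two lane components.
; Tick serves as the spawn timer: each tick spawns a random vehicle at a random lane's transform, then re-randomizes the actor's tick interval.
; Roughly a quarter of ticks also play a car sound at a randomly picked lane.
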(event `self.ReceiveBeginPlay`
  (set `self.cars` (`|MakeArray` (`self.police`) (`self.regCar`) (`self.truck`)))
  (set `self.carLanes` (`|MakeArray` (`self.car1`) (`self.car2`)))
  (`self.SetActorTickInterval` (`KismetMathLibrary.RandomFloatInRange` 3.0 15.0)))

(event `self.ReceiveTick`
  (params (DeltaSeconds :type "Float (single-precision)"))
  (bind _returnvalue (`SceneComponent.K2_GetComponentToWorld` (`KismetArrayLibrary.Array_Random` (`self.carLanes`))))
  (`|SpawnActorFromClass` (`KismetArrayLibrary.Array_Random` (`self.cars`)) _returnvalue "Undefined" "OverrideRootScale" null null)
  (`self.SetActorTickInterval` (`KismetMathLibrary.RandomFloatInRange` 3.0 15.0))
  (if (> (`KismetMathLibrary.RandomIntegerInRange` 0 100) 75)
    (`GameplayStatics.PlaySoundAtLocation` "/Game/Sounds/car.car" (.location _returnvalue) (struct) 1.0 1.0 0.0 null null null null)))

(fn `UserConstructionScript`)