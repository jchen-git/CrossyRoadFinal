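; Lane spawner actor that procedurally builds a endless-runner style track of grass, road, water and rail lanes ahead of the player.
; BeginPlay lays an initial strip behind the spawn point, narrowing the random pick to grass or road after the first few lanes.
; Each player overlap advances the actor by a random number of lane steps, spawning one lane per step.
; A FlipFlop alternates grass with hazards, favoring road or water over rail.
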(event `self.ReceiveBeginPlay`
  ;[1 1 1] Initialize Level
  (set `self.lanes` (`|MakeArray` (`self.grass`) (`self.road`) (`self.water`) (`self.rail`)))
  (set `self.startSpawnLoc` (+ (`SceneComponent.K2_GetComponentLocation` (`self.spawnLoc`)) (-1800.0 0.0 0.0)))
  (for _index (range 10)
    (`|SpawnActorFromClass` (`|GetArrayItem` (`self.lanes`) (`KismetMathLibrary.RandomIntegerInRange` 0 (`self.spawnRange`))) (`KismetMathLibrary.Conv_VectorToTransform` (+ (`self.startSpawnLoc`) (0.0 0.0 -55.0))) "Undefined" "OverrideRootScale" null null)
    (set `self.startSpawnLoc` (+ (`self.startSpawnLoc`) (200.0 0.0 0.0)))
    (if (> _index 1)
      (set `self.spawnRange` 1))))

(event `self.ReceiveActorBeginOverlap`
  (params (OtherActor :type "Actor Object Reference"))
  ;[1 1 1] Spawn Lanes
  (cast `/Game/Blueprints/player_1` OtherActor)
  (for _ (range (+ (`KismetMathLibrary.RandomIntegerInRange` (`self.minLanesSpawn`) (`self.maxLanesSpawn`)) 1))
    (`self.K2_AddActorLocalOffset` (200.0 0.0 0.0))
    (`/Engine/EditorBlueprintResources/StandardMacros.FlipFlop`
      (:`A`
        (`|SpawnActorFromClass` "/Game/Blueprints/grassTile.grassTile_C" (`KismetMathLibrary.Conv_VectorToTransform` (+ (`SceneComponent.K2_GetComponentLocation` (`self.spawnLoc`)) (0.0 0.0 -55.0))) "Undefined" "OverrideRootScale" null null))
      (:`B`
        (if (`KismetMathLibrary.InRange_FloatFloat` (`KismetMathLibrary.RandomFloatInRange` 0.0 1.0) 0.0 0.8)
          (`|SpawnActorFromClass` (`|GetArrayItem` (`self.lanes`) (`KismetMathLibrary.RandomIntegerInRange` 1 2)) (`KismetMathLibrary.Conv_VectorToTransform` (+ (`SceneComponent.K2_GetComponentLocation` (`self.spawnLoc`)) (0.0 0.0 -55.0))) "Undefined" "OverrideRootScale" null null)
          (else
            (`|SpawnActorFromClass` "/Game/Blueprints/rail.rail_C" (`KismetMathLibrary.Conv_VectorToTransform` (+ (`SceneComponent.K2_GetComponentLocation` (`self.spawnLoc`)) (0.0 0.0 -55.0))) "Undefined" "OverrideRootScale" null null)))))))

(fn `UserConstructionScript`)